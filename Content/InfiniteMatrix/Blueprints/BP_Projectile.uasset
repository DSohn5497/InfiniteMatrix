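; BP_Projectile is a short-lived projectile that destroys itself when its box overlaps another box component or its two-second life span ends.
; On BeginPlay it casts the player pawn to BP_Player and caches references to it and its health bar.
; It then adds the player's ForwardSpeed on world X to its own velocity and applies the result to its ProjectileMovement component.
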(event OnComponentBeginOverlap(Box)
  (params (OverlappedComponent :type Primitive%20Component%20Object%20Reference) (OtherActor :type Actor%20Object%20Reference) (OtherComp :type Primitive%20Component%20Object%20Reference) (OtherBodyIndex :type Integer) (bFromSweep :type Boolean) (SweepResult :type Hit%20Result%20Structure%20%28by%20ref%29))
  ;[1 1 1] Destroy projectile after collision or short amount of time
  (Utilities|Casting|CastToBoxComponent OtherComp)
  (Actor|DestroyActor))

(event EventBeginPlay
  ;[1 1 1] Destroy projectile after collision or short amount of time
  (bind _asbp_player (Utilities|Casting|CastToBP_Player (Game|Player|GetPlayerPawn 0)))
  (Variables|Default|SetPlayerRef _asbp_player)
  (Actor|SetLifeSpan 2.0)
  (Variables|/Script/Engine.MovementComponent|SetVelocity (Variables|Default|GetProjectileMovement) (+ (Transformation|GetVelocity) (Math|Vector|MakeVector (Variables|/Game/InfiniteMatrix/Blueprints/BP_Player.BP_Player_C|GetForwardSpeed _asbp_player) 0.0 0.0)))
  (Variables|Default|SetHealthBarRefFromProj (Variables|/Game/InfiniteMatrix/Blueprints/BP_Player.BP_Player_C|GetHealthBarReference _asbp_player)))

(event Collision|EventActorBeginOverlap
  (params (OtherActor :type Actor%20Object%20Reference)))

(event EventTick
  (params (DeltaSeconds :type Float%20%28single-precision%29)))

(fn ConstructionScript)