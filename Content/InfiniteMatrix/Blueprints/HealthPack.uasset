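; Health pickup actor that restores player health and destroys itself when collected, or expires after a short lifespan set on BeginPlay.
; Its box overlap accepts either BP_Player directly or a BP_Projectile, so shooting the pack also heals the player who fired it.
; Either path adds a fixed amount clamped to the health range, then refreshes the health bar through the reference held on the player or projectile.
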(event OnComponentBeginOverlap(Box)
  (params (OverlappedComponent :type Primitive%20Component%20Object%20Reference) (OtherActor :type Actor%20Object%20Reference) (OtherComp :type Primitive%20Component%20Object%20Reference) (OtherBodyIndex :type Integer) (bFromSweep :type Boolean) (SweepResult :type Hit%20Result%20Structure%20%28by%20ref%29))
  (bind _asbp_player (Utilities|Casting|CastToBP_Player OtherActor)
    (:then
      (Variables|/Game/InfiniteMatrix/Blueprints/BP_Player.BP_Player_C|SetHealth _asbp_player (Math|Float|Clamp(Float) (+ (Variables|/Game/InfiniteMatrix/Blueprints/BP_Player.BP_Player_C|GetHealth _asbp_player) 2e+01) 0.0 1e+02))
      (Default|UpdateHealthBar (Variables|/Game/InfiniteMatrix/Blueprints/BP_Player.BP_Player_C|GetHealthBarReference _asbp_player) (Variables|/Game/InfiniteMatrix/Blueprints/BP_Player.BP_Player_C|GetHealth _asbp_player))
      (Actor|DestroyActor))
    (:CastFailed
      (bind _asbp_projectile (Utilities|Casting|CastToBP_Projectile OtherActor))
      (Variables|/Game/InfiniteMatrix/Blueprints/BP_Player.BP_Player_C|SetHealth (Variables|/Game/InfiniteMatrix/Blueprints/BP_Projectile.BP_Projectile_C|GetPlayerRef _asbp_projectile) (Math|Float|Clamp(Float) (+ (Variables|/Game/InfiniteMatrix/Blueprints/BP_Player.BP_Player_C|GetHealth (Variables|/Game/InfiniteMatrix/Blueprints/BP_Projectile.BP_Projectile_C|GetPlayerRef _asbp_projectile)) 2e+01) 0.0 1e+02))
      (Default|UpdateHealthBar (Variables|/Game/InfiniteMatrix/Blueprints/BP_Projectile.BP_Projectile_C|GetHealthBarRefFromProj _asbp_projectile) (Variables|/Game/InfiniteMatrix/Blueprints/BP_Player.BP_Player_C|GetHealth (Variables|/Game/InfiniteMatrix/Blueprints/BP_Projectile.BP_Projectile_C|GetPlayerRef _asbp_projectile)))
      (Actor|DestroyActor))))

(event EventBeginPlay
  (Actor|SetLifeSpan 4.0))

(event Collision|EventActorBeginOverlap
  (params (OtherActor :type Actor%20Object%20Reference)))

(event EventTick
  (params (DeltaSeconds :type Float%20%28single-precision%29)))

(fn ConstructionScript)